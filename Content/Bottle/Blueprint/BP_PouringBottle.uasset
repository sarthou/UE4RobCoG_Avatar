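; BP_PouringBottle is a bottle that pours vinegar particles when tilted and leaves splash decals on surfaces they hit.
; Tick starts the pour when roll or pitch passes a threshold that rises as Fill drains, until empty.
; Continuous pouring grows LeakingTime, while bottle movement shrinks it.
; Particle collisions line trace along velocity to attach M_Splash decals sized by LeakingTime, so steady pours make bigger splashes.
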(event `self.ReceiveBeginPlay`
  (set `self.InitialLocation` (`SceneComponent.K2_GetComponentLocation` (`self.StaticMeshComponent`))))

(event `self.ReceiveTick`
  (params (DeltaSeconds :type "Float (single-precision)"))
  (bind _vinegar (`self.Vinegar`))
  (if (`self.Empty`)
    (`ActorComponent.Deactivate` _vinegar :!label _label)
    (set `self.LeakingTime` 0.0)
    (set `self.InitialLocation` (`SceneComponent.K2_GetComponentLocation` (`self.StaticMeshComponent`)))
    (elif (>= (`KismetMathLibrary.FMax` (`KismetMathLibrary.Abs` (.roll (`SceneComponent.K2_GetComponentRotation` (`self.StaticMeshComponent`)))) (`KismetMathLibrary.Abs` (.pitch (`SceneComponent.K2_GetComponentRotation` (`self.StaticMeshComponent`))))) (- (+ 100.0 (`self.StartLeak`)) (`self.Fill`)))
      (`ActorComponent.Activate` _vinegar false)
      (bind _output_get (set `self.Fill` (- (`self.Fill`) (* DeltaSeconds 5.0))))
      (if (> _output_get 0.0)
        (bind _output_get_2 (set `self.LeakingTime` (+ DeltaSeconds (`self.LeakingTime`))))
        (if (> _output_get_2 0.0)
          (set `self.LeakingTime` (`KismetMathLibrary.FClamp` (- _output_get_2 (`KismetMathLibrary.FClamp` (`KismetMathLibrary.Abs` (- (+ (`KismetMathLibrary.Abs` (.x (`self.InitialLocation`))) (`KismetMathLibrary.Abs` (.y (`self.InitialLocation`))) (`KismetMathLibrary.Abs` (.z (`self.InitialLocation`)))) (+ (`KismetMathLibrary.Abs` (.x (`SceneComponent.K2_GetComponentLocation` (`self.StaticMeshComponent`)))) (`KismetMathLibrary.Abs` (.y (`SceneComponent.K2_GetComponentLocation` (`self.StaticMeshComponent`)))) (`KismetMathLibrary.Abs` (.z (`SceneComponent.K2_GetComponentLocation` (`self.StaticMeshComponent`))))))))) 0.0 1000.0))
          (set `self.InitialLocation` (`SceneComponent.K2_GetComponentLocation` (`self.StaticMeshComponent`)))
          (bind _output_get_3 (set `self.Debug_Percentage_Speed` (* (`self.Max_Speed`) (- 1.0 (* (/ (`KismetMathLibrary.FMax` (`KismetMathLibrary.Abs` (.roll (`SceneComponent.K2_GetComponentRotation` (`self.StaticMeshComponent`)))) (`KismetMathLibrary.Abs` (.pitch (`SceneComponent.K2_GetComponentRotation` (`self.StaticMeshComponent`))))) 180.0) (`KismetMathLibrary.Abs` (/ (`self.Fill`) 100.0))))))))
        (else
          (set `self.Empty` true)
          (set `self.LeakingTime` 0.0)))
      (else
        (goto _label)))))

(event `self.Vinegar.OnParticleCollide`
  (params (EventName :type Name) (EmitterTime :type "Float (single-precision)") (ParticleTime :type Integer) (Location :type "Vector Structure") (Velocity :type "Vector Structure") (Direction :type "Vector Structure") (Normal :type "Vector Structure") (BoneName :type Name) (PhysMat :type "PhysicalMaterial Object Reference"))
  (bind _leakingtime (`self.LeakingTime`))
  (bind (_outhit _returnvalue) (`KismetSystemLibrary.LineTraceSingleForObjects` Location (+ Location Velocity) (`|MakeArray` "ObjectTypeQuery1" "ObjectTypeQuery2" "ObjectTypeQuery4" :!type "EObjectTypeQuery Enum")))
  (if _returnvalue
    (bind (_bblockinghit _binitialoverlap _time _distance _location _impactpoint _normal _impactnormal _physmat _hitactor _hitcomponent) (`GameplayStatics.BreakHitResult` _outhit))
    (`GameplayStatics.SpawnDecalAttached` "/Game/Bottle/Material/M_Splash.M_Splash" (* (`KismetMathLibrary.MakeVector` _leakingtime _leakingtime _leakingtime) 3) _hitcomponent "None" _location (`KismetMathLibrary.FindLookAtRotation` _location (`SceneComponent.K2_GetComponentLocation` (`self.Vinegar`))) "KeepWorldPosition")))

(fn `UserConstructionScript`)